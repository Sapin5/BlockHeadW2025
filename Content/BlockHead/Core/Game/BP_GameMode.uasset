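; BlockHead game mode that runs the level flow: HUD, level completion, restarts and the win/lose end screen.
; On BeginPlay it creates the HUD and has the cached game instance set game-only input.
; LevelComplete shows a widget, then a timer calls LoadNextLevel, which passes the HUD score to the game instance and opens the next level.
; On the final level it switches to UI input and calls GameComplete instead.
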(event `self.ReceiveBeginPlay`
  (`|ExecutionSequence`
    (:`then_0`
      ;[0.03119 1 0.1322 0.5] Add Hud To ViewPort
      (bind _returnvalue (`|GenericCreateObject` "/Game/BlockHead/Core/UI/WBP_HUD.WBP_HUD_C"))
      (bind _output_get (set `self.HUD` _returnvalue))
      (`UserWidget.AddToViewport` _output_get 0))
    (:`then_1`
      ;[0.03119 1 0.1322 0.5] Hide Mouse Pointer and Capture Keyboard
      (bind _asbp_game_instnance (cast `/Game/BlockHead/Core/Game/BP_GameInstnance` (`GameplayStatics.GetGameInstance`)))
      (set `self.Game Instnance` _asbp_game_instnance))
    (:`then_2`
      ;[0.03119 1 0.1322 0.5] Disable mouse
      (`/Game/BlockHead/Core/Game/BP_GameInstnance.InputModeGame` (`self.Game Instnance`)))))

(fn `GameComplete`
  (params (bPlayerWon :type Boolean))
  ;[0.03119 1 0.1322 0.5] Display End Screen
  (if bPlayerWon
    (set `self.WinLose` "You Win!")
    (else
      (set `self.WinLose` "You Lose :(")))
  (bind _returnvalue (`|CreateWidget` "/Game/BlockHead/Core/UI/WBP_EndGame.WBP_EndGame_C"))
  (`UserWidget.AddToViewport` _returnvalue 0)
  (set `TextBlock.Text` (`self.WinLose`) (`/Game/BlockHead/Core/UI/WBP_EndGame.WinOrLose` _returnvalue)))

(fn `LevelComplete`
  ;[0.03119 1 0.1322 0.5] In Progress
  (bind _returnvalue (`|CreateWidget` "/Game/BlockHead/Core/UI/WBP_LevelComplete.WBP_LevelComplete_C"))
  (`UserWidget.AddToViewport` _returnvalue 0)
  (`KismetSystemLibrary.K2_SetTimer` null "LoadNextLevel" 2.0)
  (return))

(fn `LoadNextLevel`
  (bind _game_instnance (`self.Game Instnance`))
  ;[0 1 0.1145 0.5] Level Completed
  ;;[0.03119 1 0.1322 0.5] Load next level and save players score
  (bind _output_get (set `self.GMScore` (`/Game/BlockHead/Core/UI/WBP_HUD.WBPScore` (`self.HUD`))))
  (if (`/Game/BlockHead/Core/Game/BP_GameInstnance.IsPlayerOnFinalLevel` (`self.Game Instnance`))
    ;;[0 1 0.1145 0.5] Player has completed level and is at the final level
    (`/Game/BlockHead/Core/Game/BP_GameInstnance.InputModeUI` (`self.Game Instnance`) false)
    (`self.GameComplete` true)
    (else
      ;;[0 1 0.1145 0.5] Player has completed level and is not at the final level
      (`/Game/BlockHead/Core/Game/BP_GameInstnance.NextLevel` _game_instnance _output_get)
      (bind _newparam (`/Game/BlockHead/Core/Game/BP_GameInstnance.GetLevelName` _game_instnance))
      (`GameplayStatics.OpenLevel` _newparam)))
  (return))

(fn `RestartGame`
  (`/Game/BlockHead/Core/Game/BP_GameInstnance.ResetInstance` (`self.Game Instnance`))
  (bind _newparam (`/Game/BlockHead/Core/Game/BP_GameInstnance.GetLevelName` (`self.Game Instnance`)))
  (`GameplayStatics.OpenLevel` _newparam))

(fn `UserConstructionScript`)